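; Player character Blueprint, a child class that adds the reaction to being caught by the Neighbor.
; Getting caught shows the WinLockerNEW widget, switches to the Mute sound mix for two seconds before restoring UnMute, and removes any BPW_Blackout widgets almost immediately.
; BeginPlay runs the parent logic and sets the UnMute mix.
; A Trace helper line-traces forward from the camera on the Visibility channel, with timed debug drawing.
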(event `self.ReceiveBeginPlay`
  (`parent.ReceiveBeginPlay`)
  (`GameplayStatics.SetBaseSoundMix` "/Hello_Veseley_2/Sound/Huesos/UnMute.UnMute"))

(event `self.OnNeighborCatchPlayer`
  (`|ExecutionSequence`
    (:`then_0`
      (bind _returnvalue (`|CreateWidget` "/Hello_Veseley_2/Widget/WinLockerNEW.WinLockerNEW_C"))
      (`UserWidget.AddToViewport` _returnvalue 0)
      (`GameplayStatics.SetBaseSoundMix` "/Hello_Veseley_2/Sound/Huesos/Mute.Mute")
      (`KismetSystemLibrary.Delay` 2.0)
      (`GameplayStatics.SetBaseSoundMix` "/Hello_Veseley_2/Sound/Huesos/UnMute.UnMute"))
    (:`then_1`
      (`KismetSystemLibrary.Delay` 0.01)
      (bind _foundwidgets (`WidgetBlueprintLibrary.GetAllWidgetsOfClass` "/Game/UMG/BPW_Blackout.BPW_Blackout_C" false))
      (for _array_element _foundwidgets
        (`Widget.RemoveFromParent` _array_element)))))

(fn `Trace`
  (params (Distance :type "Float (double-precision)"))
  (returns (OutHit :type "HitResult Structure") (ReturnValue :type Boolean))
  (bind _camera (`self.Camera`))
  (bind _returnvalue (`SceneComponent.K2_GetComponentLocation` _camera))
  (bind (_outhit _returnvalue_2) (`KismetSystemLibrary.LineTraceSingle` :`Start` _returnvalue :`End` (+ _returnvalue (* (`SceneComponent.GetForwardVector` _camera) Distance)) :`TraceChannel` "TraceTypeQuery1" :`DrawDebugType` "ForDuration"))
  (return _outhit _returnvalue_2))

(fn `UserConstructionScript`
  (`parent.UserConstructionScript`))