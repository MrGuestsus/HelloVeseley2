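; BP_Pult is an interactable remote that toggles between on and off and detonates a linked Bomb.
; The action event (E key, per the comment) flips the tumbler state.
; Each state change refreshes the spot light and mesh material, then triggers the Bomb's explosion, whether switching on or off.
; The construction script applies the same visual update, and every component counts as an action target.
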(event `self.OnEventAction`
  (params (ActionMaker :type "Actor Object Reference") (SpecialComponent :type "PrimitiveComponent Object Reference"))
  ;[1 1 1] Нажали Е
  (switch `ETumblerState` (`self.GetTumblerState`)
    (:`TUMBLER_ON`
      (`self.SetTumblerState` "TUMBLER_OFF"))
    (:`TUMBLER_OFF`
      (`self.SetTumblerState` "TUMBLER_ON"))))

(event `self.OnChangeTumblerState`
  (params (NewState :type "ETumblerState Enum" :default "TUMBLER_ON"))
  ;[1 1 1] Изменилось состояние фонарика
  (switch `ETumblerState` NewState
    (:`TUMBLER_ON`
      _)
    (:`TUMBLER_OFF`
      _))
  (`self.UpdateData`)
  (`/Hello_Veseley_2/BP_Object/BP_BombHV2.ВзРЫВАЕМСЯ НАХУЙ` (`self.Bomb`)))

(fn `OnIsActionComponent`
  (params (Component :type "PrimitiveComponent Object Reference"))
  (returns (Result :type Boolean))
  (return true))

(fn `UpdateData`
  (bind _spotcomponent (`self.SpotComponent`))
  (bind _staticmeshcomponent (`self.StaticMeshComponent`))
  (switch `ETumblerState` (`self.GetTumblerState`)
    (:`TUMBLER_ON`
      (`SceneComponent.SetVisibility` _spotcomponent true false)
      (`PrimitiveComponent.SetMaterial` _staticmeshcomponent 0 "/Game/Objects/Materials/instances/flashlight_on_inst.flashlight_on_inst"))
    (:`TUMBLER_OFF`
      (`SceneComponent.SetVisibility` _spotcomponent false false)
      (`PrimitiveComponent.SetMaterial` _staticmeshcomponent 0 "/Game/Objects/Materials/Base/Base_mirror.base_mirror"))))

(fn `UserConstructionScript`
  (`self.UpdateData`))