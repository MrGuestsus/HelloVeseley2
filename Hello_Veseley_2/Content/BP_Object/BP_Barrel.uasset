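; Heavy explosive barrel actor that catches fire and detonates after rough collisions or an external Explode call.
; Fast overlaps adjust BarrelHealf from both speeds (own speed adds health), and low health starts fire, light and a random-delay fuse, which StopFire cancels.
; Detonation notifies FindSosed's tutorial check, enlarges the sphere, plays effects, fires a radial impulse and destroys the barrel.
; Sphere overlap is empty, leaving barrel-to-barrel chain-reaction logic unconnected.
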(event `self.ReceiveBeginPlay`
  (`PrimitiveComponent.SetMassOverrideInKg` (`self.StaticMeshComponent`) "None" 600.0 true))

(event `self.ReceiveActorBeginOverlap`
  (params (OtherActor :type "Actor Object Reference"))
  (bind _returnvalue (`KismetMathLibrary.VSize` (`self.GetVelocity`)))
  (bind _returnvalue_2 (`KismetMathLibrary.VSize` (`self.GetVelocity` OtherActor)))
  (if (or (> _returnvalue_2 200.0) (> _returnvalue 200.0))
    (bind _output_get (set `self.barrel_healf` (+ (- (`self.barrel_healf`) (/ _returnvalue_2 6.0)) (/ _returnvalue 6.0))))
    (if (<= _output_get 25.0)
      (`SceneComponent.SetVisibility` (`self.PointLight`) true false :!label _label)
      (`ActorComponent.Activate` (`self.P_Fire`) false)
      (bind _returnvalue_3 (`KismetSystemLibrary.K2_SetTimerDelegate` (delegate `Detonation`) (`KismetMathLibrary.RandomFloatInRange` 0.7 2.2)))
      (set `self.Timer` _returnvalue_3))))

(event `Explode`
  (goto _label))

(event `Detonation`
  (bind _sphere (`self.Sphere`))
  (bind _staticmeshcomponent (`self.StaticMeshComponent`))
  (`ActorComponent.Activate` (`self.BOOOM`) false)
  (`/Engine/EditorBlueprintResources/StandardMacros.IsValid` self
    (:`Is Valid`
      (bind _returnvalue (`Sosed.FindSosed`))
      (`Sosed.TutorialCheckObject` _returnvalue self)
      (`/Engine/EditorBlueprintResources/StandardMacros.IsValid` _sphere
        (:`Is Valid`
          (`SphereComponent.SetSphereRadius` _sphere 700.0 true)
          (`ActorComponent.Activate` (`self.P_Explosion_Thing`) false)
          (set `self.Взорваллась?` true)
          (`/Engine/EditorBlueprintResources/StandardMacros.IsValid` _staticmeshcomponent
            (:`Is Valid`
              (`ActorComponent.K2_DestroyComponent` _staticmeshcomponent)
              (`RadialForceComponent.FireImpulse` (`self.RadialForce`))
              (`KismetSystemLibrary.Delay` 0.2)
              (`ActorComponent.Deactivate` (`self.P_Fire`))
              (`SceneComponent.SetVisibility` (`self.PointLight`) false false)
              (`KismetSystemLibrary.Delay` 2.0)
              (`self.K2_DestroyActor`))))))))

(event `self.Sphere.OnComponentBeginOverlap`
  (params (OverlappedComponent :type "PrimitiveComponent Object Reference") (OtherActor :type "Actor Object Reference") (OtherComp :type "PrimitiveComponent Object Reference") (OtherBodyIndex :type Integer) (bFromSweep :type Boolean) (SweepResult :type "HitResult Structure (by ref)")))

(event `StopFire`
  (`KismetSystemLibrary.K2_ClearAndInvalidateTimerHandle` (`self.Timer`))
  (`SceneComponent.SetVisibility` (`self.PointLight`) false false)
  (`ActorComponent.Deactivate` (`self.P_Fire`)))

(event `self.Box.OnComponentBeginOverlap`
  (params (OverlappedComponent :type "PrimitiveComponent Object Reference") (OtherActor :type "Actor Object Reference") (OtherComp :type "PrimitiveComponent Object Reference") (OtherBodyIndex :type Integer) (bFromSweep :type Boolean) (SweepResult :type "HitResult Structure (by ref)")))

(fn `OnIsActionComponent`
  (params (Component :type "PrimitiveComponent Object Reference"))
  (returns (Result :type Boolean))
  (return true))

(fn `UserConstructionScript`)