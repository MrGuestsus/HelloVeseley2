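; BP_Airplane is an airplane actor that flies straight ahead dropping bombs and destroys itself after 25 seconds.
; Tick moves it a fixed step along the Arrow component's forward vector without sweep, so its speed depends on frame rate.
; From BeginPlay, a looping Delay spawns a Bomba at the Scene component every 0.6 seconds and launches its mesh along Arrow1 with a velocity-change impulse.
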(event `self.ReceiveBeginPlay`
  (`|ExecutionSequence`
    (:`then_0`
      (`KismetSystemLibrary.Delay` 25.0)
      (`self.K2_DestroyActor`))
    (:`then_1`
      (bind _returnvalue (`|SpawnActorFromClass` "/Hello_Veseley_2/BP_Object/Bomba.Bomba_C" (`KismetMathLibrary.Conv_VectorToTransform` (`SceneComponent.K2_GetComponentLocation` (`self.Scene`))) "Undefined" "OverrideRootScale" null null :!label _label))
      (`PrimitiveComponent.AddImpulse` (`/Hello_Veseley_2/BP_Object/Bomba.StaticMesh` _returnvalue) (* (`SceneComponent.GetForwardVector` (`self.Arrow1`)) 4000.0) "None" true)
      (`KismetSystemLibrary.Delay` 0.6)
      (goto _label))))

(event `self.ReceiveTick`
  (params (DeltaSeconds :type "Float (single-precision)"))
  (`self.K2_SetActorLocation` (+ (`self.K2_GetActorLocation`) (* (`SceneComponent.GetForwardVector` (`self.Arrow`)) 10.0)) false true))

(fn `UserConstructionScript`)