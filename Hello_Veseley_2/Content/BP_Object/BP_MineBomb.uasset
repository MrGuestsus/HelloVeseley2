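; BP_MineBomb is a mine object that explodes once when something triggers its box overlap.
; A FlatActor triggers it only while its static mesh simulates physics, while a Human or Sosed always does.
; Detonation plays a destruction sound, fires a radial force impulse and spawns an explosion emitter.
; It then reports itself to the Sosed for a tutorial check and, after a zero-length delay, sets its FlatComponent to Delete mode.
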(event `self.Box.OnComponentBeginOverlap`
  (params (OverlappedComponent :type "PrimitiveComponent Object Reference") (OtherActor :type "Actor Object Reference") (OtherComp :type "PrimitiveComponent Object Reference") (OtherBodyIndex :type Integer) (bFromSweep :type Boolean) (SweepResult :type "HitResult Structure (by ref)"))
  (bind _returnvalue (`self.K2_GetActorLocation`))
  (bind _asflat_actor (cast `FlatActor` OtherActor)
    (:`then`
      (if (`SceneComponent.IsSimulatingPhysics` (`self.GetComponentByClass` _asflat_actor "/Script/Engine.StaticMeshComponent") "None")
        (`/Engine/EditorBlueprintResources/StandardMacros.DoOnce` false :!label _label
          (:`Completed`
            (`GameplayStatics.PlaySoundAtLocation` "/Game/Sounds/Maps/FinalBattle/house_destruction_Cue.house_destruction_Cue" _returnvalue (struct) 1.0 1.0 0.0 null null null)
            (`RadialForceComponent.FireImpulse` (`self.RadialForce`))
            (`GameplayStatics.SpawnEmitterAtLocation` "/Game/Effects/Particle/P_Explosion_Bomb.P_Explosion_Bomb" _returnvalue (struct))
            (bind _returnvalue_2 (`Sosed.FindSosed`))
            (`Sosed.TutorialCheckObject` _returnvalue_2 self)
            (`KismetSystemLibrary.Delay` 0.0)
            (`FlatComponent.SetMode` (`self.FlatComponent`) "FM_Delete")))))
    (:`CastFailed`
      (cast `Human` OtherActor
        (:`then`
          (goto _label))
        (:`CastFailed`
          (cast `Sosed` OtherActor)
          (goto _label))))))

(fn `UserConstructionScript`)