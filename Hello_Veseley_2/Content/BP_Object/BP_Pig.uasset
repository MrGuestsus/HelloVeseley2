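; BP_Pig is a wandering pig pawn that explodes when a Human walks into it.
; On BeginPlay it loops AI move-to requests to random reachable points within a radius around itself, pausing briefly after each success or failure.
; Its Box overlap casts the other actor to Human, then spawns BP_Explode and a pig sound at its location and destroys the pig.
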(event `self.ReceiveBeginPlay`
  (`|AIMoveTo` self (`NavigationSystemV1.K2_GetRandomReachablePointInRadius` (`self.K2_GetActorLocation`) 1500.0 null null) null :!label _label
    (:`OnSuccess`
      _)
    (:`OnFail`
      _))
  (`KismetSystemLibrary.Delay` 2.0)
  (goto _label))

(event `self.Box.OnComponentBeginOverlap`
  (params (OverlappedComponent :type "PrimitiveComponent Object Reference") (OtherActor :type "Actor Object Reference") (OtherComp :type "PrimitiveComponent Object Reference") (OtherBodyIndex :type Integer) (bFromSweep :type Boolean) (SweepResult :type "HitResult Structure (by ref)"))
  ;[1 1 1] AS
  (cast `Human` OtherActor)
  (`|SpawnActorFromClass` "/Hello_Veseley_2/BP_Object/BP_Explode.BP_Explode_C" (`self.GetTransform`) "Undefined" "OverrideRootScale" null null)
  (`GameplayStatics.SpawnSoundAtLocation` "/Hello_Veseley_2/Sound/pIG/pig-1__1__Cue.pig-1__1__Cue" (`self.K2_GetActorLocation`) (struct) 1.0 1.0 0.0 null null)
  (`KismetSystemLibrary.Delay` 0.0)
  (`self.K2_DestroyActor`))

(fn `UserConstructionScript`)