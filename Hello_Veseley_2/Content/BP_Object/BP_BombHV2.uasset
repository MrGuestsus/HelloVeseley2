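; BP_BombHV2 is a grabbable bomb that the player character can plant on surfaces and that explodes through a separate event.
; Applying it while held traces from BP_HumanStupid2, plays a throw hand state, and fixes the bomb at the impact point with rotation derived from the hit normal.
; Grabbing resets its planted flags and rotation.
; The one-shot explosion fires effects, hides the mesh, applies a radial impulse, then destroys the actor.
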(event `self.Apply.OnApply`
  (params (ApplyActor :type "Actor Object Reference") (TraceActor :type "FlatActor Object Reference") (TraceComponent :type "PrimitiveComponent Object Reference"))
  (bind _returnvalue (`Human.FindHuman`))
  (bind _asbp_human_stupid_2 (cast `/Hello_Veseley_2/Human/BP_HumanStupid2` _returnvalue))
  (bind (_outhit _returnvalue_2) (`/Hello_Veseley_2/Human/BP_HumanStupid2.Trace` _asbp_human_stupid_2 300.0))
  (if _returnvalue_2
    (`GameplayStatics.PlaySound2D` null 1.0 1.0 0.0 null null)
    (bind _returnvalue_3 (`Human.GetInventory` _asbp_human_stupid_2))
    (if (== (`Inventory.GetCurrentObject` _returnvalue_3) self)
      (`Human.SetHandsState` _asbp_human_stupid_2 "HS_FAST_THROW")
      (`KismetSystemLibrary.Delay` 0.0)
      (`FlatComponent.SetMode` (`self.FlatComponent`) "FM_Fixed")
      (`SceneComponent.K2_SetWorldRotation` :`self` (`self.StaticMeshComponent`))
      (set `self.Поставил ли обомбу` true)
      (bind (_bblockinghit _binitialoverlap _time _distance _location _impactpoint _normal) (`GameplayStatics.BreakHitResult` _outhit))
      (bind (_returnvalue_roll _returnvalue_pitch _returnvalue_yaw) (`KismetMathLibrary.BreakRotator` (`KismetMathLibrary.MakeRotFromXY` _normal _impactpoint)))
      (`self.K2_SetActorTransform` (`KismetMathLibrary.MakeTransform` _impactpoint (`KismetMathLibrary.MakeRotator` _returnvalue_pitch _returnvalue_yaw))))))

(event `self.OnGrab`
  (params (Character :type "Actor Object Reference"))
  (set `self.Поставил ли обомбу` false)
  (set `self.В боксе` false)
  (`self.K2_SetActorRotation` (struct :`Pitch` 90.0)))

(event `ВзРЫВАЕМСЯ НАХУЙ`
  (`/Engine/EditorBlueprintResources/StandardMacros.DoOnce` false
    (:`Completed`
      (set `self.В боксе` true)
      (`ActorComponent.Activate` (`self.P_Explosion_Bomb`) false)
      (`ActorComponent.Activate` (`self.c4_explode1_Cue`) false)
      (`KismetSystemLibrary.Delay` 0.06)
      (`SceneComponent.SetVisibility` (`self.StaticMeshComponent`) false false)
      (`SphereComponent.SetSphereRadius` (`self.Sphere`) 1500.0 true)
      (`RadialForceComponent.FireImpulse` (`self.RadialForce`))
      (`KismetSystemLibrary.Delay` 2.0)
      (`self.K2_DestroyActor`))))

(fn `OnIsActionComponent`
  (params (Component :type "PrimitiveComponent Object Reference"))
  (returns (Result :type Boolean))
  (return true))

(fn `UserConstructionScript`)