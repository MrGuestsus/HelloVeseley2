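; BP_Svinoferma is a pig farm spawner that keeps the level stocked with BP_Pig AI pawns.
; Every Tick it counts all BP_Pig actors in the world and spawns one whenever there are fewer than ten.
; The spawn location builds X, Y and Z from separate random reachable-point queries around the farm, each with a random radius, then lifts Z slightly, so the combined point may not itself be reachable.
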(event `self.ReceiveTick`
  (params (DeltaSeconds :type "Float (single-precision)"))
  (bind _outactors (`GameplayStatics.GetAllActorsOfClass` "/Hello_Veseley_2/BP_Object/BP_Pig.BP_Pig_C"))
  (if (not (> (`KismetArrayLibrary.Array_LastIndex` _outactors) 8))
    (`AIBlueprintHelperLibrary.SpawnAIFromClass` "/Hello_Veseley_2/BP_Object/BP_Pig.BP_Pig_C" null (`KismetMathLibrary.MakeVector` (.x (`NavigationSystemV1.K2_GetRandomReachablePointInRadius` (`self.K2_GetActorLocation`) (`KismetMathLibrary.RandomFloatInRange` 100.0 600.0) null null)) (.y (`NavigationSystemV1.K2_GetRandomReachablePointInRadius` (`self.K2_GetActorLocation`) (`KismetMathLibrary.RandomFloatInRange` 100.0 600.0) null null)) (+ (.z (`NavigationSystemV1.K2_GetRandomReachablePointInRadius` (`self.K2_GetActorLocation`) (`KismetMathLibrary.RandomFloatInRange` 100.0 600.0) null null)) 50.0)))))

(fn `UserConstructionScript`)