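; BP_Vazilochka_20 is a cart the player boards through a one-time action event.
; On action it hides and deactivates the human, attaches it to Scene, aligns its controller, switches view and input to itself, and reveals its skeletal mesh.
; Turn-axis input then rotates the cart camera within clamped pitch and yaw limits.
; The graph contains no exit or movement logic, despite its "Cart moving" comment and Move flag.
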(event `InputAxis|InputTurnX` :consume false
  (params (AxisValue :type "Float (single-precision)"))
  (bind (_returnvalue_roll _returnvalue_pitch _returnvalue_yaw) (`KismetMathLibrary.BreakRotator` (`KismetMathLibrary.ComposeRotators` (`KismetMathLibrary.MakeRotator` 0.0 0.0 AxisValue) (`self.RotationCamera`))))
  (if (> (`KismetMathLibrary.Abs` AxisValue) 0.0)
    (bind _output_get (set `self.RotationCamera` (`KismetMathLibrary.MakeRotator` 0.0 _returnvalue_pitch (`KismetMathLibrary.ClampAngle` _returnvalue_yaw 120.0 240.0))))
    (`SceneComponent.K2_SetRelativeRotation` (`self.Camera`) _output_get false false)))

(event `InputAxis|InputTurnY` :consume false
  (params (AxisValue :type "Float (single-precision)"))
  (bind (_returnvalue_roll _returnvalue_pitch _returnvalue_yaw) (`KismetMathLibrary.BreakRotator` (`KismetMathLibrary.ComposeRotators` (`KismetMathLibrary.MakeRotator` 0.0 (* AxisValue -1.0)) (`self.RotationCamera`))))
  (if (> (`KismetMathLibrary.Abs` AxisValue) 0.0)
    (bind _output_get (set `self.RotationCamera` (`KismetMathLibrary.MakeRotator` 0.0 (`KismetMathLibrary.ClampAngle` _returnvalue_pitch -60.0 60.0) _returnvalue_yaw)))
    (`SceneComponent.K2_SetRelativeRotation` (`self.Camera`) _output_get false false)))

(event `self.OnEventAction`
  (params (ActionMaker :type "Actor Object Reference") (SpecialComponent :type "PrimitiveComponent Object Reference"))
  (bind _returnvalue (`GameplayStatics.GetPlayerController` 0))
  (bind _scene (`self.Scene`))
  (`/Engine/EditorBlueprintResources/StandardMacros.DoOnce` false
    (:`Completed`
      (`Human.FindHuman`)
      ;[1 1 1] Cart moving
      (if (not (`self.bMove`))
        (set `self.bMove` true)
        (bind _returnvalue_2 (`Human.FindHuman`))
        (`Human.DeActive` _returnvalue_2 true false)
        (`self.K2_AttachToComponent` _returnvalue_2 _scene "None" "SnapToTarget" "SnapToTarget" "KeepRelative" false)
        (`Controller.SetControlRotation` (`Pawn.GetController` _returnvalue_2) (`SceneComponent.K2_GetComponentRotation` _scene))
        (`PlayerController.SetViewTargetWithBlend` _returnvalue self 0.0 "VTBlend_Linear" 0.0 false)
        (`self.EnableInput` _returnvalue)
        (`SceneComponent.SetHiddenInGame` (`self.SkeletalMesh`) false true)
        (set `self.RotationCamera` (`SceneComponent.RelativeRotation` (`self.Camera`)))))))

(fn `UserConstructionScript`)