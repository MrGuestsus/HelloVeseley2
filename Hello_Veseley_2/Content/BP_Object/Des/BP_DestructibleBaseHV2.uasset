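; Base physics prop that takes impact damage and is replaced by a spawned destructible actor when its HP runs out.
; Hits apply damage from component velocity, with a second check adding the other body's mass, each throttled by a resetting DoOnce.
; Destruction spawns the replacement, optionally adds a simulated destructible mesh, then removes the prop.
; Fire activation switches a holder's hands to fast-throw, and burning disables the action component.
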(event `self.ReceiveBeginPlay`
  (`PrimitiveComponent.SetMassOverrideInKg` (`self.StaticMeshComponent`) "None" (`self.MassKG`) true))

(event `Destructible`
  (bind _returnvalue (`SceneComponent.K2_GetComponentToWorld` (`self.StaticMeshComponent`)))
  (`KismetSystemLibrary.PrintString` "Des" true true (struct :`R` 1.0 :`G` 0.096302 :`A` 1.0))
  (`/Engine/EditorBlueprintResources/StandardMacros.DoOnce` false
    (:`Completed`
      (set `self.SpeedD` (`self.GetActorForwardVector`))
      (bind _returnvalue_2 (`|SpawnActorFromClass` (`self.DestructibleActor`) _returnvalue "Undefined" "OverrideRootScale" null null))
      (set `/Hello_Veseley_2/BP_Object/Des/DestructibleHV2.Parent` self _returnvalue_2)
      (`|ExecutionSequence`
        (:`then_0`
          (if (`self.old?`)
            (bind _returnvalue_3 (`AddComponent|NODE_AddDestructibleComponent-0` :`self` _returnvalue_2))
            (`DestructibleComponent.SetDestructibleMesh` _returnvalue_3 (`self.DestructibleMesh`))
            (`PrimitiveComponent.SetSimulatePhysics` _returnvalue_3 true)
            (`PrimitiveComponent.SetMaterial` _returnvalue_3 0 (`PrimitiveComponent.GetMaterial` (`self.Mesh`) 0))
            (`self.K2_SetActorTransform` _returnvalue_2 _returnvalue false false)
            (`self.K2_DestroyActor`)
            (else
              (`self.K2_DestroyActor`))))))))

(event `self.ReceiveHit`
  (params (MyComp :type "PrimitiveComponent Object Reference") (Other :type "Actor Object Reference") (OtherComp :type "PrimitiveComponent Object Reference") (bSelfMoved :type Boolean) (HitLocation :type "Vector Structure") (HitNormal :type "Vector Structure") (NormalImpulse :type "Vector Structure") (Hit :type "HitResult Structure (by ref)"))
  (bind _returnvalue (`KismetMathLibrary.VSize` (`SceneComponent.GetComponentVelocity` MyComp)))
  (bind _returnvalue_2 (>= _returnvalue 30.0))
  (bind _returnvalue_3 (/ _returnvalue 20.0))
  (bind _returnvalue_4 (`KismetMathLibrary.FCeil` _returnvalue_3))
  (bind _returnvalue_5 (`KismetMathLibrary.FCeil` (+ _returnvalue_3 (/ (`PrimitiveComponent.GetMass` OtherComp) 6.0))))
  (bind _returnvalue_6 (`KismetMathLibrary.Conv_IntToDouble` _returnvalue_4))
  (bind _returnvalue_7 (`KismetMathLibrary.Conv_IntToDouble` _returnvalue_5))
  (`|ExecutionSequence`
    (:`then_0`
      (if (and _returnvalue_2 (>= _returnvalue_6 20.0))
        (`/Engine/EditorBlueprintResources/StandardMacros.DoOnce` false :!label _label
          (:`Completed`
            (`self.Damage` _returnvalue_6)
            (`KismetSystemLibrary.Delay` 0.6)
            (`KismetSystemLibrary.PrintString` (`KismetStringLibrary.Conv_IntToString` _returnvalue_5) false)
            (goto _label :!via `Reset`)))))
    (:`then_1`
      (if (and _returnvalue_2 (>= _returnvalue_7 10.0))
        (`/Engine/EditorBlueprintResources/StandardMacros.DoOnce` false :!label _label_2
          (:`Completed`
            (`self.Damage` _returnvalue_7)
            (`KismetSystemLibrary.Delay` 0.6)
            (`KismetSystemLibrary.PrintString` (`KismetStringLibrary.Conv_IntToString` _returnvalue_4) false)
            (goto _label_2 :!via `Reset`)))))))

(event `self.P_Fire.OnComponentActivated`
  (params (Component :type "ActorComponent Object Reference") (bReset :type Boolean))
  (bind _returnvalue (`Human.FindHuman`))
  (bind _returnvalue_2 (`Human.GetInventory` _returnvalue))
  (if (== (`Inventory.GetCurrentObject` _returnvalue_2) self)
    (`Human.SetHandsState` _returnvalue "HS_FAST_THROW")))

(fn `Damage`
  (params (Damage :type "Float (double-precision)"))
  (bind _output_get (set `self.HP` (- (`self.HP`) Damage)))
  (if (<= _output_get 0.0)
    (`self.Destructible`)
    (else
      (return))))

(fn `OnIsActionComponent`
  (params (Component :type "PrimitiveComponent Object Reference"))
  (returns (Result :type Boolean))
  (return (not (`self.Burn?`))))

(fn `UserConstructionScript`)