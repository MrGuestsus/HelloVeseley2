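; BP_ChairDM is a chair prop that can be grabbed and responds to blocking or unblocking a door.
; Block and unblock events play the PropDoorCloseCue and PropDoorOpenCue sounds, and grabbing plays a 2D chair pick-up sound.
; OnIsActionComponent returns true for any component passed to it.
; The blueprint adds only this feedback, and BeginPlay just calls its parent.
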(event `self.ReceiveBeginPlay`
  (`parent.ReceiveBeginPlay`))

(event `OnBlockDoor`
  (params (BlockedDoor :type "Door Object Reference"))
  (`AudioComponent.Play` (`self.prop_door_close_Cue`) 0.0))

(event `OnUnblockDoor`
  (`AudioComponent.Play` (`self.prop_door_open_Cue`) 0.0))

(event `self.OnGrab`
  (params (Character :type "Actor Object Reference"))
  (`GameplayStatics.PlaySound2D` "/Hello_Uzbek/Soand/UP/chair_pick_up_1_Cue.chair_pick_up_1_Cue" 1.0 1.0 0.0 null null))

(fn `OnIsActionComponent`
  (params (Component :type "PrimitiveComponent Object Reference"))
  (returns (Result :type Boolean))
  (return true))

(fn `UserConstructionScript`)